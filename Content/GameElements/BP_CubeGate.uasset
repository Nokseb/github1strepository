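; BP_CubeGate is a trigger box that animates track elements when the player vehicle overlaps it.
; On the first overlap, a DoOnce picks a BP_ObstacleByLap from the level and a timeline offsets its location, setting a flag that it is up.
; A Gate node also lets a second timeline yaw the first BP_Gate found, closing itself as the rotation updates.
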(event `self.BoxDetectionOfObstacles.OnComponentBeginOverlap`
  (params (OverlappedComponent :type "PrimitiveComponent Object Reference") (OtherActor :type "Actor Object Reference") (OtherComp :type "PrimitiveComponent Object Reference") (OtherBodyIndex :type Integer) (bFromSweep :type Boolean) (SweepResult :type "HitResult Structure (by ref)"))
  (bind (_relativerotation_roll _relativerotation_pitch _relativerotation_yaw) (`KismetMathLibrary.BreakRotator` (`SceneComponent.RelativeRotation` (`/Game/GameElements/BP_Gate.Cylinder` (`self.Gate`)))))
  (cast `/Game/Player/BP_PlayerVehicule` OtherActor)
  (`|ExecutionSequence`
    (:`then_0`
      (if (not (`self.bYellowCylinderUp?`))
        (`/Engine/EditorBlueprintResources/StandardMacros.DoOnce` false
          (:`Completed`
            (bind _outactors (`GameplayStatics.GetAllActorsOfClass` "/Game/GameElements/BP_ObstacleByLap.BP_ObstacleByLap_C"))
            (bind _output_get (set `self.YellowCylinderObstacle` _outactors))
            (for _index (range (+ (`self.Array Index`) 1)) :!label _label
              (bind _output_get_2 (set `self.Array Index` _index))
              (if (== _output_get_2 (`self.Array Index`))
                (`KismetSystemLibrary.PrintString` (`KismetStringLibrary.Conv_IntToString` _output_get_2))
                (else
                  (`self.StopNVisible`))))
            (bind _output (`|GetArrayItem` _output_get _output_get_2))
            (set `self.YellowCylinder` (`self.K2_GetActorLocation` _output))
            (bind (_direction _newtrack_1) (`Timeline|Timeline`)
              (:`Update`
                (`self.K2_SetActorRelativeLocation` _output (+ _newtrack_1 (`self.YellowCylinder`)) false false)
                (set `self.bYellowCylinderUp?` true)))))))
    (:`then_1`
      (`self.Open`)
      (`/Engine/EditorBlueprintResources/StandardMacros.Gate` true :!label _label_2
        (:`Exit`
          (bind _outactors_2 (`GameplayStatics.GetAllActorsOfClass` "/Game/GameElements/BP_Gate.BP_Gate_C"))
          (bind _output_2 (`|GetArrayItem` _outactors_2))
          (set `self.Gate` _output_2)
          (bind (_direction_2 _newtrack_0) (`Timeline|TimeLineGate`)
            (:`Update`
              (`self.K2_SetActorRelativeRotation` _output_2 (`KismetMathLibrary.MakeRotator` _relativerotation_roll _relativerotation_pitch (+ _newtrack_0 _relativerotation_yaw)) false false)
              (`self.Close`))))))))

(event `StopNVisible`
  (goto _label :!via `Break`))

(event `Open`
  (goto _label_2 :!via `Open`))

(event `Close`
  (goto _label_2 :!via `Close`))

(event `ActivateOpenOrClose`
  (goto _label_2 :!via `Toggle`))

(fn `UserConstructionScript`)