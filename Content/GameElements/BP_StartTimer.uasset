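; BP_StartTimer is the race start/finish trigger that times the player vehicle's run and counts laps up to three.
; The first StartNFinish overlap starts a looping one-second timer and briefly hides the trigger.
; A FlipFlop alternates start and finish checks; finishing with three laps recorded prints the time, stops the timer and quits.
; A separate BoxDoOnceWall overlap moves the first BP_WallStopInStart actor once via Timeline.
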(event `self.StartNFinish.OnComponentBeginOverlap`
  (params (OverlappedComponent :type "PrimitiveComponent Object Reference") (OtherActor :type "Actor Object Reference") (OtherComp :type "PrimitiveComponent Object Reference") (OtherBodyIndex :type Integer) (bFromSweep :type Boolean) (SweepResult :type "HitResult Structure (by ref)"))
  (cast `/Game/Player/BP_PlayerVehicule` OtherActor)
  (`|ExecutionSequence`
    (:`then_0`
      (if (== (`self.NumberOfLaps`) 3)
        (set `self.NumberLapCondition` true)
        (else
          (set `self.NumberLapCondition` false)))
      (`/Engine/EditorBlueprintResources/StandardMacros.FlipFlop`
        (:`A`
          (if (not (`self.bStartGo`))
            (`self.Timer`)
            (`SceneComponent.SetVisibility` (`self.StartNFinish`) false false)
            (`KismetSystemLibrary.Delay` 2.0)
            (`SceneComponent.SetVisibility` (`self.StartNFinish`) true false)
            (set `self.bStartGo` true)))
        (:`B`
          (if (and (`self.bStartGo`) (`self.NumberLapCondition`))
            (`SceneComponent.SetVisibility` (`self.StartNFinish`) false false)
            (`KismetSystemLibrary.Delay` 2.0)
            (`SceneComponent.SetVisibility` (`self.StartNFinish`) true false)
            (set `self.bStartGo` false)
            (`KismetSystemLibrary.PrintString` (`KismetStringLibrary.Conv_IntToString` (`self.Second`)) true true (struct :`R` 1.0 :`B` 0.617609 :`A` 1.0) 20.0)
            (`KismetSystemLibrary.K2_ClearAndInvalidateTimerHandle` (stale `Timer` _returnvalue))
            (`KismetSystemLibrary.Delay` 3.0)
            (`KismetSystemLibrary.QuitGame` null "Quit")))))
    (:`then_1`
      (bind _counter (`/Engine/EditorBlueprintResources/StandardMacros.Do N` 3)
        (:`Exit`
          (bind _output_get (set `self.NumberOfLaps` _counter))
          (`KismetSystemLibrary.PrintString` (`KismetStringLibrary.Conv_IntToString` _output_get)))))))

(event `Timer`
  (bind _returnvalue (`KismetSystemLibrary.K2_SetTimerDelegate` (delegate `Add1s`) 1.0 true)))

(event `Add1s`
  (bind _result (`/Engine/EditorBlueprintResources/StandardMacros.IncrementInt` (`self.Second`))
    (:`  `
      (bind _output_get (set `self.Second` _result))
      (`KismetSystemLibrary.PrintString` (`KismetStringLibrary.Conv_IntToString` _output_get) true true (struct :`R` 0.234375 :`A` 1.0) 0.8))))

(event `self.BoxDoOnceWall.OnComponentBeginOverlap`
  (params (OverlappedComponent :type "PrimitiveComponent Object Reference") (OtherActor :type "Actor Object Reference") (OtherComp :type "PrimitiveComponent Object Reference") (OtherBodyIndex :type Integer) (bFromSweep :type Boolean) (SweepResult :type "HitResult Structure (by ref)"))
  (cast `/Game/Player/BP_PlayerVehicule` OtherActor)
  (`/Engine/EditorBlueprintResources/StandardMacros.DoOnce` false
    (:`Completed`
      (bind _outactors (`GameplayStatics.GetAllActorsOfClass` "/Game/GameElements/BP_WallStopInStart.BP_WallStopInStart_C"))
      (bind _output_get (set `self.WallStart` (`|GetArrayItem` _outactors)))
      (set `self.WallStopLocation` (`self.K2_GetActorLocation` _output_get))
      (bind (_direction _newtrack_1) (`Timeline|Timeline`)
        (:`Update`
          (`self.K2_SetActorRelativeLocation` (`self.WallStart`) (+ _newtrack_1 (`self.WallStopLocation`)) false false))))))

(fn `UserConstructionScript`)