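; Gate actor that rotates its Cylinder when a BP_PlayerVehicule enters its Sphere trigger.
; Overlap stores the Cylinder's rotation, then opens and enters a flow-control Gate; end overlap closes it.
; Each pass applies a single RInterpTo step, with no Tick or Timeline, toward a rotation built from the Cylinder's X-offset world location, inverse-transformed as a direction into actor space.
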(event `GateOpen`
  (bind (_returnvalue_x _returnvalue_y _returnvalue_z) (`KismetMathLibrary.BreakVector` (`SceneComponent.K2_GetComponentLocation` (`self.Cylinder`))))
  (`|ExecutionSequence`
    (:`then_0`
      (goto _label :!via `Open`))
    (:`then_1`
      (`/Engine/EditorBlueprintResources/StandardMacros.Gate` true :!label _label
        (:`Exit`
          (`SceneComponent.K2_SetRelativeRotation` (`self.Cylinder`) (`KismetMathLibrary.RInterpTo` (`self.Relative Rotation`) (`KismetMathLibrary.MakeRotFromX` (`KismetMathLibrary.InverseTransformDirection` (`self.GetTransform`) (`KismetMathLibrary.MakeVector` (+ _returnvalue_x 1000.0) _returnvalue_y _returnvalue_z))) (`GameplayStatics.GetWorldDeltaSeconds`) 20.0) false false))))))

(event `self.Sphere.OnComponentBeginOverlap`
  (params (OverlappedComponent :type "PrimitiveComponent Object Reference") (OtherActor :type "Actor Object Reference") (OtherComp :type "PrimitiveComponent Object Reference") (OtherBodyIndex :type Integer) (bFromSweep :type Boolean) (SweepResult :type "HitResult Structure (by ref)"))
  (cast `/Game/Player/BP_PlayerVehicule` OtherActor)
  (set `self.Relative Rotation` (`SceneComponent.RelativeRotation` (`self.Cylinder`)))
  (`self.GateOpen`))

(event `CloseGate`
  (goto _label :!via `Close`))

(event `ToggleGate`
  (goto _label :!via `Toggle`))

(event `self.Sphere.OnComponentEndOverlap`
  (params (OverlappedComponent :type "PrimitiveComponent Object Reference") (OtherActor :type "Actor Object Reference") (OtherComp :type "PrimitiveComponent Object Reference") (OtherBodyIndex :type Integer))
  (cast `/Game/Player/BP_PlayerVehicule` OtherActor)
  (`self.CloseGate`))

(fn `UserConstructionScript`)